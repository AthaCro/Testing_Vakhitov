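; BP_balls_dead is a functional test that checks where the play ball is when it dies.
; On test start it casts the player pawn to boat, stores the boat cube's world location and binds to the ball's CallOnDead dispatcher.
; When that fires, the test succeeds if the ball's X is below the boat's starting X and fails otherwise.
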(event Custom|CustomEvent_0
  (if (< (.x (Transformation|GetWorldLocation (Variables|/Game/bp_ball.bp_ball_C|GetSphere (Variables|Default|GetPlay%20Ball)))) (.x (Variables|Default|Getboat_location)))
    (Class|FunctionalTest|FinishTest "Succeeded")
    (else
      (Class|FunctionalTest|FinishTest "Failed"))))

(event EventPrepareTest)

(event EventStartTest
  (bind _asboat (Utilities|Casting|CastToboat (Game|Player|GetPlayerPawn 0)))
  (Variables|Default|Setboat_location (Transformation|GetWorldLocation (Variables|/Game/boat.boat_C|GetCube _asboat)))
  (bind _output_get (Variables|Default|SetPlay%20Ball (Variables|/Game/boat.boat_C|GetplayBall _asboat)))
  (EventDispatchers|BindEventtoCallonDead _output_get (delegate Custom|CustomEvent_0)))

(event EventTick
  (params (DeltaSeconds :type Float%20%28single-precision%29)))

(fn ConstructionScript)