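; Ball actor that moves at a set speed and bounces off whatever blocks it, until it enters a KillZVolume.
; Tick moves it with a swept world offset along Direction, scaled by Speed and delta time.
; On a blocking hit, GetReflectionVector computes a new Direction from the surface normal, with Z forced to zero to keep travel planar.
; Overlapping a KillZVolume fires the OnDead dispatcher and destroys the ball.
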(event Collision|EventActorBeginOverlap
  (params (OtherActor :type Actor%20Object%20Reference))
  (Utilities|Casting|CastToKillZVolume OtherActor)
  (Default|CallCallonDead)
  (Actor|DestroyActor))

(event EventTick
  (params (DeltaSeconds :type Float%20%28single-precision%29))
  (bind _sweephitresult (Transformation|AddActorWorldOffset (* (* (Variables|Default|Getdirection) (Variables|Default|Getspeed)) DeltaSeconds) true))
  (if (.bBlockingHit (Collision|BreakHitResult _sweephitresult))
    (Variables|Default|Setdirection (Math|Vector|MakeVector (.x (Math|Vector|GetReflectionVector (Math|Vector|MakeVector (.x (Variables|Default|Getdirection)) (.y (Variables|Default|Getdirection)) 0.0) (Math|Vector|MakeVector (.x (.Normal (Collision|BreakHitResult _sweephitresult))) (.y (.Normal (Collision|BreakHitResult _sweephitresult))) 0.0))) (.y (Math|Vector|GetReflectionVector (Math|Vector|MakeVector (.x (Variables|Default|Getdirection)) (.y (Variables|Default|Getdirection)) 0.0) (Math|Vector|MakeVector (.x (.Normal (Collision|BreakHitResult _sweephitresult))) (.y (.Normal (Collision|BreakHitResult _sweephitresult))) 0.0))) 0.0))))

(fn ConstructionScript)